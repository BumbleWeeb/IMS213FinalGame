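; Lockable rock door that moves vertically when BP_FirstPersonCharacter overlaps it while unlocked.
; It starts locked; eventUnlockDoor clears the lock and, after a short delay, switches the indicator light's material.
; Two timelines offset the rock from its starting height, with a falling-stones sound.
; An overlap runs LowerDoor when the door is down and idle, and RaiseDoor only when it is already moving.
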(event `Lower Door`
  (set `self.doorisUp` false)
  (bind (_direction _garagedoorheight) (`Timeline|Lower the door` :!via `PlayFromStart`)
    (:`Update`
      (`SceneComponent.K2_SetWorldLocation` (`self.S_Nordic_Forest_Rock_Moss_Large_xetmcci_lod3_Var1`) (`KismetMathLibrary.MakeVector` (`self.StartX`) (`self.StartY`) (+ _garagedoorheight (`self.StartZ`))) false false))
    (:`Finished`
      (set `self.doorisDown` true)
      (set `self.doorisMoving` false))))

(event `Raise Door`
  (set `self.doorisDown` false)
  (bind (_direction _garagedoorheight) (`Timeline|Raise the door` :!via `PlayFromStart`)
    (:`Update`
      (`SceneComponent.K2_SetWorldLocation` (`self.S_Nordic_Forest_Rock_Moss_Large_xetmcci_lod3_Var1`) (`KismetMathLibrary.MakeVector` (`self.StartX`) (`self.StartY`) (+ _garagedoorheight (`self.StartZ`))) false false))
    (:`Finished`
      (set `self.doorisUp` true)
      (set `self.doorisMoving` false))))

(event `self.ReceiveActorBeginOverlap`
  (params (OtherActor :type "Actor Object Reference"))
  (cast `/Game/FirstPerson/Blueprints/BP_FirstPersonCharacter` OtherActor)
  (if (`self.doorisLocked`)
    _
    (elif (`self.doorisMoving`)
      (set `self.doorisMoving` true)
      (`GameplayStatics.PlaySound2D` "/Game/MyContent/Assets/stones-falling-6375.stones-falling-6375" 1.0 1.0 0.0 null null)
      (`self.Raise Door`)
      (elif (`self.doorisDown`)
        (set `self.doorisMoving` true)
        (`GameplayStatics.PlaySound2D` "/Game/MyContent/Assets/stones-falling-6375.stones-falling-6375" 1.0 1.0 0.0 null null)
        (`self.Lower Door`)))))

(event `self.ReceiveBeginPlay`
  (bind (_returnvalue_x _returnvalue_y _returnvalue_z) (`KismetMathLibrary.BreakVector` (`SceneComponent.K2_GetComponentLocation` (`self.S_Nordic_Forest_Rock_Moss_Large_xetmcci_lod3_Var1`))))
  (set `self.StartX` _returnvalue_x)
  (set `self.StartY` _returnvalue_y)
  (set `self.StartZ` _returnvalue_z)
  (set `self.doorisDown` true)
  (set `self.doorisUp` false)
  (set `self.doorisMoving` false)
  (set `self.doorisLocked` true)
  (`PrimitiveComponent.SetMaterial` (`self.Statis Light`) 0 "/Game/MyContent/Assets/M_Door_Lock.M_Door_Lock"))

(event `eventUnlockDoor`
  (set `self.doorisLocked` false)
  (`KismetSystemLibrary.Delay` 0.75)
  (`PrimitiveComponent.SetMaterial` (`self.Statis Light`) 0 "/Game/MyContent/Assets/m_Door_Unlock.m_Door_Unlock"))

(fn `UserConstructionScript`)